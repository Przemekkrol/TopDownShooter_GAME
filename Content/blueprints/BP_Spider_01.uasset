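; BP_Spider_01 is a spider enemy that chases the player and attacks at close range.
; An AIMoveTo loop started on BeginPlay repeats shortly after each success, with no retry on failure.
; Each Tick, a living spider within AttackRange plays its attack montage, pausing CharacterMovement until completion.
; AnyDamage lowers clamped health and sets DeadSpider at zero, which blocks attacks but leaves the chase loop untouched.
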(event `self.ReceiveAnyDamage`
  (params (Damage :type "Float (single-precision)") (DamageType :type "DamageType Object Reference") (InstigatedBy :type "Controller Object Reference") (DamageCauser :type "Actor Object Reference"))
  ;[0 0.05984 1] damage
  (bind _output_get (set `self.Health_Spider` (`KismetMathLibrary.FClamp` (- (`self.Health_Spider`) Damage) 0.0 100.0)))
  (set `self.Dead_Spider` (== _output_get 0.0)))

(event `self.ReceiveBeginPlay`
  ;[1 0.3866 0] Movement
  (`|AIMoveTo` self (0.0 0.0 0.0) (`GameplayStatics.GetPlayerCharacter` 0) :!label _label
    (:`OnSuccess`
      (`KismetSystemLibrary.Delay` 0.2)
      (goto _label))))

(event `self.ReceiveTick`
  (params (DeltaSeconds :type "Float (single-precision)"))
  ;[0 1 0.2008] Attack
  (if (`self.Is Alive`)
    (if (and (`self.IsAttackRange`) (not (`self.IsAttacking`)))
      (`ActorComponent.Deactivate` (`self.CharacterMovement`))
      (`|PlayMontage` (`self.Mesh`) "/Game/Characters/Enemy_Great_Spider/Animations/AM_SpiderAttac.AM_SpiderAttac"
        (:`OnCompleted`
          (`ActorComponent.Activate` (`self.CharacterMovement`) false))))))

(fn `Is Alive`
  (returns (ReturnValue :type Boolean))
  (return (not (`self.Dead_Spider`))))

(fn `IsAttacking`
  (returns (ReturnValue :type Boolean))
  (return (`AnimInstance.Montage_IsPlaying` (`SkeletalMeshComponent.GetAnimInstance` (`self.Mesh`)) "/Game/Characters/Enemy_Great_Spider/Animations/AM_SpiderAttac.AM_SpiderAttac")))

(fn `IsAttackRange`
  (returns (ReturnValue :type Boolean))
  (return (< (`self.GetDistanceTo` (`GameplayStatics.GetPlayerCharacter` 0)) (`self.AttackRange`))))

(fn `UserConstructionScript`)