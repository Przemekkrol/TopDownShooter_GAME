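; Player shooter character that creates its HUD, moves along capsule axes, tracks health until death, and fires an assault rifle.
; Each tick while alive, it eases control yaw toward the mouse movement's direction once speed exceeds a dead zone.
; Fire toggles muzzle effect and sound, running one debug-drawn line trace per press from the muzzle socket along control rotation.
; The trace's ApplyDamage node is unconnected, so shots deal no damage.
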(event `self.ReceiveBeginPlay`
  ;[0 1 0.5776] HUD
  (bind _returnvalue (`|CreateWidget` "/Game/UI/W_PlayerHUD_01.W_PlayerHUD_01_C" null self))
  (`UserWidget.AddToViewport` _returnvalue 0))

(event `self.ReceiveTick`
  (params (DeltaSeconds :type "Float (single-precision)"))
  ;[1 0.02893 0] Movement
  (if (`self.IsAlive`)
    (`self.Rotate Character`)))

(event `InputAxis|MoveForwardBack`
  (params (AxisValue :type "Float (single-precision)"))
  ;[1 0.02893 0] Movement
  (if (`self.IsAlive`)
    (`self.AddMovementInput` (`SceneComponent.GetForwardVector` (`self.CapsuleComponent`)) AxisValue)))

(event `InputAxis|MoveLeftRight`
  (params (AxisValue :type "Float (single-precision)"))
  ;[1 0.02893 0] Movement
  (if (`self.IsAlive`)
    (`self.AddMovementInput` (`SceneComponent.GetRightVector` (`self.CapsuleComponent`)) AxisValue)))

(event `self.ReceiveAnyDamage`
  (params (Damage :type "Float (single-precision)") (DamageType :type "DamageType Object Reference") (InstigatedBy :type "Controller Object Reference") (DamageCauser :type "Actor Object Reference"))
  ;[1 0.6547 0.156] damage
  (bind _output_get (set `self.Health` (`KismetMathLibrary.FClamp` (- (`self.Health`) Damage) 0.0 100.0)))
  (bind _output_get_2 (set `self.Dead` (== _output_get 0.0)))
  (if _output_get_2
    (`self.StopFired`)))

(event `InputAction|Fire`
  (params (Key :type "Key Structure"))
  ;[0 0.2054 1] Weapon Fire
  (:`Pressed`
    (if (`self.IsAlive`)
      (`self.StartFired`)
      (`self.WeaponTrace`)
      (else
        (`self.StopFired` :!label _label)
        (if (`self.IsAlive`)
          (`GameplayStatics.SpawnSound2D` "/Game/Sounds/Weapon_AssaultRifle/Stereo/SC_WeaponFireEnd.SC_WeaponFireEnd" 1.0 1.0 0.0 null)))))
  (:`Released`
    (goto _label)))

(fn `Get Start Location LT`
  (returns (ReturnValue :type "Vector Structure"))
  (return (`SceneComponent.GetSocketLocation` (`self.Weapon`) "P_AssaultRifle_MF")))

(fn `GetEndLocationLT`
  (returns (ReturnValue :type "Vector Structure"))
  (return (+ (`self.Get Start Location LT`) (* (`KismetMathLibrary.GetForwardVector` (`self.GetControlRotation`)) (`self.WeaponRange`)))))

(fn `IsAlive`
  (returns (ReturnValue :type Boolean))
  (return (not (`self.Dead`))))

(fn `IsMouseDeadZone`
  (returns (ReturnValue :type Boolean))
  (return (> (`KismetMathLibrary.VSize2D` (`self.MouseVelocity`)) (`self.DeadZone`))))

(fn `MouseVelocity`
  (returns (ReturnValue :type "Vector2D Structure"))
  (bind (_deltax _deltay) (`PlayerController.GetInputMouseDelta` (`GameplayStatics.GetPlayerController` 0)))
  (return (/ (`KismetMathLibrary.MakeVector2D` _deltax _deltay) (`GameplayStatics.GetWorldDeltaSeconds`))))

(fn `Rotate Character`
  (bind _returnvalue (`GameplayStatics.GetPlayerController` 0))
  (bind (_returnvalue_x _returnvalue_y) (`KismetMathLibrary.BreakVector2D` (`self.MouseVelocity`)))
  (if (`self.IsMouseDeadZone`)
    (`Controller.SetControlRotation` _returnvalue (`KismetMathLibrary.RInterpTo` (`Controller.GetControlRotation` _returnvalue) (`KismetMathLibrary.MakeRotator` 0.0 0.0 (`KismetMathLibrary.DegAtan2` _returnvalue_x _returnvalue_y)) (`GameplayStatics.GetWorldDeltaSeconds`) (`self.Interp Speed`)))))

(fn `StartFired`
  (`ActorComponent.Activate` (`self.P_AssaultRifle_MF`) false)
  (bind _returnvalue (`GameplayStatics.SpawnSound2D` "/Game/Sounds/Weapon_AssaultRifle/Stereo/SC_WeaponFire.SC_WeaponFire" 1.0 1.0 0.0 null))
  (set `self.Weapon Sound` _returnvalue))

(fn `StopFired`
  (bind _weapon_sound (`self.Weapon Sound`))
  (`ActorComponent.Deactivate` (`self.P_AssaultRifle_MF`))
  (`/Engine/EditorBlueprintResources/StandardMacros.IsValid` _weapon_sound
    (:`Is Valid`
      (`AudioComponent.Stop` _weapon_sound))))

(fn `UserConstructionScript`)

(fn `WeaponTrace`
  (bind _outhit (`KismetSystemLibrary.LineTraceSingle` :`Start` (`self.Get Start Location LT`) :`End` (`self.GetEndLocationLT`) :`TraceChannel` "TraceTypeQuery1" :`DrawDebugType` "ForDuration")))